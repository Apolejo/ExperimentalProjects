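; Level actor for a bubble-shooter that owns the staggered bubble grid as a Tile map from coordinates to bubbles.
; BeginPlay builds the grid, draws debug axes and spawns bubbles from a custom map or randomly.
; SnapBubble places bubbles, then uses PlayerActor searches to break matches of three or more and floating clusters.
; Every few turns, bubbles shift one column and a new line spawns; passing column zero or snapping onto an occupied cell triggers GameOver.
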(event `self.ReceiveBeginPlay`
  (set `self.LevelX` (`KismetMathLibrary.Conv_IntToDouble` (* (`self.TileWidth`) (`self.Columns`))))
  (set `self.LevelY` (`KismetMathLibrary.Conv_IntToDouble` (* (`self.RowHeight`) (`self.Rows`))))
  (`self.RenderTiles`))

(event `RenderTiles`
  (for _index (range (+ (`self.Rows`) 1))
    (for _index_2 (range (+ (`self.Columns`) 1))
      (`BlueprintMapLibrary.Map_Add` (`self.Tile`) (`KismetMathLibrary.MakeVector2D` (`KismetMathLibrary.Conv_IntToDouble` _index_2) (`KismetMathLibrary.Conv_IntToDouble` _index))) ; Tile+Type
      (bind (_tile_x _tile_y) (`self.GetTileCoordinate` _index_2 _index))
      (bind _output_get (set `self.Coord` (`KismetMathLibrary.MakeVector2D` (`KismetMathLibrary.Conv_IntToDouble` _tile_x) (`KismetMathLibrary.Conv_IntToDouble` _tile_y)))) ; CurrentWorldCoordinate
      (bind (_x _y) (`KismetMathLibrary.BreakVector2D` _output_get))
      (`KismetSystemLibrary.DrawDebugCoordinateSystem` (`KismetMathLibrary.MakeVector` _x _y) (struct) 1.0 30.0 10.0)))
  (`self.AddBubbles` (- (`self.StartingBubbles`) 1) (`self.UsingCustomMap`)))

(event `SnapBubble`
  (params (BubbleActor :type "/Game/BubblePop_Template/Blueprints/BP_Bubble Object Reference"))
  (`self.SnapBubbleToGrid` BubbleActor))

(fn `AddBubbles`
  (params (LinesToBeAdded :type Integer) (`Using Tile_Row Matrix` :type Boolean))
  (locals (Local_Bubble :type "/Game/BubblePop_Template/Blueprints/BP_Bubble Object Reference"))
  (bind _tile_custom (`self.Tile_Custom`))
  (if `Using Tile_Row Matrix`
    (bind _keys (`BlueprintMapLibrary.Map_Keys` _tile_custom))
    (for _array_element _keys
      (bind (_x _y) (`KismetMathLibrary.BreakVector2D` _array_element))
      (bind (_tile_x _tile_y) (`self.GetTileCoordinate` (`KismetMathLibrary.FTrunc` _x) (`KismetMathLibrary.FTrunc` _y)))
      (bind _returnvalue (`|SpawnActorFromClass` "/Game/BubblePop_Template/Blueprints/BP_Bubble.BP_Bubble_C" (`KismetMathLibrary.MakeTransform` (`KismetMathLibrary.MakeVector` (`KismetMathLibrary.Conv_IntToDouble` _tile_x) (`KismetMathLibrary.Conv_IntToDouble` _tile_y))) "Undefined" "OverrideRootScale" null 0.0 false self (`BlueprintMapLibrary.Map_Find` _tile_custom _array_element) null))
      (bind _output_get (set `local.Local_Bubble` _returnvalue))
      (bind _output_get_2 (set `/Game/BubblePop_Template/Blueprints/BP_Bubble.GridPosition` _array_element _output_get))
      (`BlueprintMapLibrary.Map_Add` (`self.Tile`) _output_get_2 _output_get))
    (else
      (for _index (range (+ (`self.Rows`) 1))
        (for _index_2 (range (+ LinesToBeAdded 1))
          (bind _returnvalue_2 (- (`self.Columns`) _index_2))
          (bind (_tile_x_2 _tile_y_2) (`self.GetTileCoordinate` _returnvalue_2 _index))
          (bind _returnvalue_3 (`|SpawnActorFromClass` "/Game/BubblePop_Template/Blueprints/BP_Bubble.BP_Bubble_C" (`KismetMathLibrary.MakeTransform` (`KismetMathLibrary.MakeVector` (`KismetMathLibrary.Conv_IntToDouble` _tile_x_2) (`KismetMathLibrary.Conv_IntToDouble` _tile_y_2))) "Undefined" "OverrideRootScale" null 0.0 false self (select `int` (`KismetMathLibrary.RandomInteger` (`self.MaxRandomColorSpawn`)) :`0` "NewEnumerator0" :`1` "NewEnumerator1" :`2` "NewEnumerator2" :`3` "NewEnumerator3" :`4` "NewEnumerator4" :`5` "NewEnumerator5" :!type "/Game/BubblePop_Template/Blueprints/Bubble_Type Enum") null))
          (bind _output_get_3 (set `local.Local_Bubble` _returnvalue_3))
          (bind _output_get_4 (set `/Game/BubblePop_Template/Blueprints/BP_Bubble.GridPosition` (`KismetMathLibrary.MakeVector2D` (`KismetMathLibrary.Conv_IntToDouble` _returnvalue_2) (`KismetMathLibrary.Conv_IntToDouble` _index)) _output_get_3))
          (`BlueprintMapLibrary.Map_Add` (`self.Tile`) _output_get_4 _output_get_3))))))

(fn `CheckGameOver`
  (returns (ReturnValue :type Boolean))
  (for _index (range (+ (`self.Rows`) 1))
    (return (`KismetSystemLibrary.IsValid` (`BlueprintMapLibrary.Map_Find` (`self.Tile`) (`KismetMathLibrary.MakeVector2D` (`KismetMathLibrary.Conv_IntToDouble` -1) (`KismetMathLibrary.Conv_IntToDouble` _index)))))))

(fn `GetGridPosition`
  (params (X :type Integer) (Y :type Integer))
  (returns (Grid_X :type Integer) (Grid_Y :type Integer))
  (locals (GridY :type Integer) (xOffSet :type Integer) (GridX :type Integer))
  (set `local.GridY` (/ Y (`self.RowHeight`)))
  (set `local.xOffSet` 0)
  (if (== (mod (+ (`local.xOffSet`) (`self.RowOffset`)) 2) 0)
    (set `local.xOffSet` (/ (`self.TileWidth`) 2)))
  (set `local.GridX` (/ (- X (`local.xOffSet`)) (`self.TileWidth`)))
  (return (`local.GridX`) (`local.GridY`)))

(fn `GetTileCoordinate`
  (params (Column :type Integer) (Row :type Integer))
  (returns (Tile_X :type Integer) (Tile_Y :type Integer))
  (locals (TileX :type Integer) (TileY :type Integer))
  (set `local.TileX` (* Column (`self.TileWidth`)))
  (if (== (mod (+ Row (`self.RowOffset`)) 2) 0)
    (set `local.TileX` (+ (`local.TileX`) (/ (`self.TileWidth`) 2))))
  (set `local.TileY` (* Row (`self.RowHeight`)))
  (return (`local.TileX`) (`local.TileY`)))

(fn `MoveDownBubbles`
  (bind _tile (`self.Tile`))
  (for _index (range (+ (`self.Rows`) 1))
    (for _index_2 (range (+ (`self.Columns`) 1))
      (bind _returnvalue (`KismetMathLibrary.Conv_IntToDouble` (- _index_2 1)))
      (bind _returnvalue_2 (`KismetMathLibrary.Conv_IntToDouble` _index))
      (bind _value (`BlueprintMapLibrary.Map_Find` _tile (`KismetMathLibrary.MakeVector2D` (`KismetMathLibrary.Conv_IntToDouble` _index_2) _returnvalue_2)))
      (`BlueprintMapLibrary.Map_Add` _tile (`KismetMathLibrary.MakeVector2D` _returnvalue _returnvalue_2) _value)
      (`/Engine/EditorBlueprintResources/StandardMacros.IsValid` _value
        (:`Is Valid`
          (bind _output_get (set `/Game/BubblePop_Template/Blueprints/BP_Bubble.GridPosition` (`KismetMathLibrary.MakeVector2D` _returnvalue _returnvalue_2) _value))
          (if (== _returnvalue -1.0)
            (bind _asbp_bubbles_controller (cast `/Game/BubblePop_Template/Blueprints/BP_Bubbles_Controller` (`GameplayStatics.GetPlayerController` 0)))
            (`/Game/BubblePop_Template/Blueprints/BP_Bubbles_Controller.GameOver` _asbp_bubbles_controller)
            (else
              (`/Game/BubblePop_Template/Blueprints/BP_Bubble.SetGridPosition` _value)))))))
  (`self.AddBubbles` 0))

(fn `SnapBubbleToGrid`
  (params (BubbleActor :type "/Game/BubblePop_Template/Blueprints/BP_Bubble Object Reference"))
  (locals (Local_Bubble_Ref :type "/Game/BubblePop_Template/Blueprints/BP_Bubble Object Reference") (Local_CenterX :type "Float (double-precision)") (Local_CenterY :type "Float (double-precision)") (Local_GridPos :type "Vector2D Structure") (Local_Clusters :type "Array of /Game/BubblePop_Template/Blueprints/BP_Bubble Object Reference") (NewRow :type Integer) (Local_AddTile :type Boolean))
  (bind (_local_gridpos_x _local_gridpos_y) (`KismetMathLibrary.BreakVector2D` (`local.Local_GridPos`)))
  (bind _local_gridpos (`local.Local_GridPos`))
  (bind (_local_gridpos_x_2 _local_gridpos_y_2) (`KismetMathLibrary.BreakVector2D` (`local.Local_GridPos`)))
  (bind (_local_gridpos_x_3 _local_gridpos_y_3) (`KismetMathLibrary.BreakVector2D` (`local.Local_GridPos`)))
  (bind (_local_gridpos_x_4 _local_gridpos_y_4) (`KismetMathLibrary.BreakVector2D` (`local.Local_GridPos`)))
  (bind _local_bubble_ref (`local.Local_Bubble_Ref`))
  (bind (_grid_x _grid_y) (`self.GetGridPosition` (`KismetMathLibrary.Round` (`local.Local_CenterX`)) (`KismetMathLibrary.Round` (`local.Local_CenterY`))))
  (bind (_tile_x _tile_y) (`self.GetTileCoordinate` (`KismetMathLibrary.FTrunc` _local_gridpos_x_2) (`KismetMathLibrary.FTrunc` _local_gridpos_y_2)))
  (bind _output_get (set `local.Local_Bubble_Ref` BubbleActor))
  (`/Engine/EditorBlueprintResources/StandardMacros.IsValid` _output_get
    (:`Is Valid`
      (bind (_returnvalue_x _returnvalue_y) (`KismetMathLibrary.BreakVector` (`self.K2_GetActorLocation` _output_get)))
      (set `local.Local_CenterX` (+ _returnvalue_x (/ (`KismetMathLibrary.Conv_IntToDouble` (`self.RowHeight`)) 2.0)))
      (set `local.Local_CenterY` (+ _returnvalue_y (/ (`KismetMathLibrary.Conv_IntToDouble` (`self.TileWidth`)) 2.0)))
      (set `local.Local_GridPos` (`KismetMathLibrary.MakeVector2D` (`KismetMathLibrary.Conv_IntToDouble` _grid_x) (`KismetMathLibrary.Conv_IntToDouble` _grid_y)))
      (if (not (`KismetSystemLibrary.IsValid` (`BlueprintMapLibrary.Map_Find` (`self.Tile`) (`KismetMathLibrary.MakeVector2D` _local_gridpos_x _local_gridpos_y))))
        ;[1 1 1] Fix Any Possible Overlap
        (bind _output_get_2 (set `local.NewRow` (`KismetMathLibrary.FTrunc` _local_gridpos_x_3)))
        (for _index (range 1 (+ _output_get_2 1))
          (if (not (`.ReturnValue` (`BlueprintMapLibrary.Map_Find` (`self.Tile`) (`KismetMathLibrary.MakeVector2D` (`KismetMathLibrary.Conv_IntToDouble` _index) _local_gridpos_y_3))))
            (set `local.Local_GridPos` (`KismetMathLibrary.MakeVector2D` _local_gridpos_x_4 _local_gridpos_y_4))
            (break)))
        (`BlueprintMapLibrary.Map_Add` (`self.Tile`) _local_gridpos _local_bubble_ref)
        (bind _output_get_3 (set `/Game/BubblePop_Template/Blueprints/BP_Bubble.GridPosition` _local_gridpos _local_bubble_ref))
        (`self.K2_SetActorLocation` _local_bubble_ref (`KismetMathLibrary.MakeVector` (`KismetMathLibrary.Conv_IntToDouble` _tile_x) (`KismetMathLibrary.Conv_IntToDouble` _tile_y)) false false)
        (bind (_x _y) (`KismetMathLibrary.BreakVector2D` _output_get_3))
        (bind _output_get_4 (set `self.Cluster` (`/Game/BubblePop_Template/Blueprints/BP_PlayerWeapon.FindCluster` (`self.PlayerActor`) _x _y true true false)))
        (if (>= (`KismetArrayLibrary.Array_Length` _output_get_4) 3)
          (for _array_element (`self.Cluster`)
            (`/Game/BubblePop_Template/Blueprints/BP_Bubble.MatchBreak` _array_element))
          (bind _output_get_5 (set `local.Local_Clusters` (`/Game/BubblePop_Template/Blueprints/BP_PlayerWeapon.FindFloatingCluster` (`self.PlayerActor`))))
          (if (> (`KismetArrayLibrary.Array_Length` _output_get_5) 0)
            (for _array_element_2 _output_get_5
              (`/Game/BubblePop_Template/Blueprints/BP_Bubble.FloatingBreak` _array_element_2))))
        (bind _outactors (`GameplayStatics.GetAllActorsOfClass` "/Game/BubblePop_Template/Blueprints/BP_Bubble.BP_Bubble_C"))
        (if (`KismetSystemLibrary.IsValid` (`|GetArrayItem` _outactors))
          (if (>= (`self.CurrentTurn`) (`self.Turns`))
            (set `self.CurrentTurn` 1)
            (`self.MoveDownBubbles`)
            (else
              (`/Engine/EditorBlueprintResources/StandardMacros.IncrementInt` (`self.CurrentTurn`)))))
        (else
          (bind _asbp_bubbles_controller (cast `/Game/BubblePop_Template/Blueprints/BP_Bubbles_Controller` (`GameplayStatics.GetPlayerController` 0)))
          (`/Game/BubblePop_Template/Blueprints/BP_Bubbles_Controller.GameOver` _asbp_bubbles_controller))))))

(fn `UserConstructionScript`)