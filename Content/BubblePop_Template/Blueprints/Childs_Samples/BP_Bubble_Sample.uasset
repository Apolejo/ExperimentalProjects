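; Sample child bubble Blueprint from the BubblePop template that demonstrates how a bubble reacts to parent-defined events.
; It handles Snapping, MatchBreak and FloatingBreak, printing a debug message for each.
; MatchBreak and FloatingBreak also destroy the actor, while Snapping only logs.
; The construction script just calls the parent, and the default BeginPlay, overlap and Tick nodes are disabled.
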(event `self.Snapping`
  (`KismetSystemLibrary.PrintString` "Hi, i did a snap"))

(event `self.MatchBreak`
  (`KismetSystemLibrary.PrintString` "Hi, im breaking")
  (`self.K2_DestroyActor`))

(event `self.FloatingBreak`
  (`KismetSystemLibrary.PrintString` "Hi, i was floating")
  (`self.K2_DestroyActor`))

(fn `UserConstructionScript`
  (`parent.UserConstructionScript`))