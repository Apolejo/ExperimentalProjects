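; Player weapon for a bubble shooter that aims at the mouse within a clamped yaw, fires on left click and loads a new random-type bubble.
; Firing is gated by CanFire, which this Blueprint never re-arms.
; It also provides grid searches over the level's tile map: a flood fill using parity-based neighbor offsets, with optional type matching.
; FindFloatingCluster reuses that fill to return clusters detached from the top edge.
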(event `SpawnBubble`
  (bind (_returnvalue_roll _returnvalue_pitch _returnvalue_yaw) (`KismetMathLibrary.BreakRotator` (`SceneComponent.K2_GetComponentRotation` (`self.LookAt`))))
  ;[0 0.09151 1] Spawn Bubble On Weapon
  (bind _returnvalue (`|SpawnActorFromClass` "/Game/BubblePop_Template/Blueprints/BP_Bubble.BP_Bubble_C" (`KismetMathLibrary.MakeTransform` (`self.K2_GetActorLocation`)) "Undefined" "OverrideRootScale" null (* _returnvalue_yaw -1.0) false (`self.Level_Ref`) (select `int` (`KismetMathLibrary.RandomInteger` (`self.PlayerMaxColorSpawn`)) :`0` "NewEnumerator0" :`1` "NewEnumerator1" :`2` "NewEnumerator2" :`3` "NewEnumerator3" :`4` "NewEnumerator4" :`5` "NewEnumerator5" :!type "/Game/BubblePop_Template/Blueprints/Bubble_Type Enum") null))
  (set `self.Bubble_Ref` _returnvalue))

(event `self.ReceiveTick`
  (params (DeltaSeconds :type "Float (single-precision)"))
  (bind (_returnvalue_roll _returnvalue_pitch) (`KismetMathLibrary.BreakRotator` (`self.K2_GetActorRotation`)))
  (bind (_angleclamp_x _angleclamp_y) (`KismetMathLibrary.BreakVector2D` (`self.AngleClamp`)))
  (bind (_worldlocation _worlddirection) (`PlayerController.DeprojectMousePositionToWorld` (`GameplayStatics.GetPlayerController` 0)))
  (bind (_returnvalue_roll_2 _returnvalue_pitch_2 _returnvalue_yaw) (`KismetMathLibrary.BreakRotator` (`KismetMathLibrary.FindLookAtRotation` (`self.K2_GetActorLocation`) (+ _worldlocation (* _worlddirection 2000.0)))))
  ;[0 1 0.5174] Set "Arrow" Rotation by Mouse Position
  (`SceneComponent.K2_SetWorldRotation` (`self.LookAt`) (`KismetMathLibrary.MakeRotator` _returnvalue_roll _returnvalue_pitch (`KismetMathLibrary.FClamp` _returnvalue_yaw _angleclamp_x _angleclamp_y)) false false))

(event `ResetProcessed`
  ;[1 1 1] Reset Processed Bubbles
  (for _index (range (+ (`/Game/BubblePop_Template/Blueprints/BP_Bubbles_Level.Columns` (`self.Level_Ref`)) 1))
    (for _index_2 (range (+ (`/Game/BubblePop_Template/Blueprints/BP_Bubbles_Level.Rows` (`self.Level_Ref`)) 1))
      (bind _value (`BlueprintMapLibrary.Map_Find` (`/Game/BubblePop_Template/Blueprints/BP_Bubbles_Level.Tile` (`self.Level_Ref`)) (`KismetMathLibrary.MakeVector2D` (`KismetMathLibrary.Conv_IntToDouble` _index) (`KismetMathLibrary.Conv_IntToDouble` _index_2))))
      (`/Engine/EditorBlueprintResources/StandardMacros.IsValid` _value
        (:`Is Valid`
          (set `/Game/BubblePop_Template/Blueprints/BP_Bubble.Processed` false _value))))))

(event `ShootBubble`
  (bind _bubble_ref (`self.Bubble_Ref`))
  (bind (_returnvalue_roll _returnvalue_pitch _returnvalue_yaw) (`KismetMathLibrary.BreakRotator` (`SceneComponent.K2_GetComponentRotation` (`self.LookAt`))))
  ;[1 1 1] Fire Weapon
  (if (`self.CanFire?`)
    (set `self.CanFire?` false)
    (`/Engine/EditorBlueprintResources/StandardMacros.IsValid` _bubble_ref
      (:`Is Valid`
        (set `/Game/BubblePop_Template/Blueprints/BP_Bubble.bFired` true _bubble_ref)
        (set `/Game/BubblePop_Template/Blueprints/BP_Bubble.Angle` (* _returnvalue_yaw -1.0) _bubble_ref)
        (`self.SpawnBubble`)))))

(event `Key|LeftMouseButton`
  (params (Key :type "Key Structure"))
  ;[1 0 0] Fire Action
  (:`Pressed`
    (`self.ShootBubble`)))

(fn `FindCluster`
  (params (tX :type "Float (double-precision)") (tY :type "Float (double-precision)") (MatchType :type Boolean) (Reset :type Boolean) (SkipRemoved :type Boolean))
  (returns (ClustersFound :type "Array of /Game/BubblePop_Template/Blueprints/BP_Bubble Object Reference"))
  (locals (ToProcess :type "Array of /Game/BubblePop_Template/Blueprints/BP_Bubble Object Reference") (TargetTile :type "/Game/BubblePop_Template/Blueprints/BP_Bubble Object Reference") (FoundCluster :type "Array of /Game/BubblePop_Template/Blueprints/BP_Bubble Object Reference") (CurrentTile :type "/Game/BubblePop_Template/Blueprints/BP_Bubble Object Reference") (Neighbors :type "Array of /Game/BubblePop_Template/Blueprints/BP_Bubble Object Reference"))
  (bind _currenttile (`local.CurrentTile`))
  (if Reset
    (`self.ResetProcessed`))
  (bind _output_get (set `local.TargetTile` (`BlueprintMapLibrary.Map_Find` (`/Game/BubblePop_Template/Blueprints/BP_Bubbles_Level.Tile` (`self.Level_Ref`)) (`KismetMathLibrary.MakeVector2D` tX tY)))) ; Current tile bubble
  (`KismetArrayLibrary.Array_Add` (`local.ToProcess`) _output_get) ; To Be Processed Array
  (set `/Game/BubblePop_Template/Blueprints/BP_Bubble.Processed` true _output_get) ; Set the current tile as processed
  (for _array_element (`local.ToProcess`)
    (bind _output_get_2 (set `local.CurrentTile` _array_element)) ; Local Tile
    (if (`KismetSystemLibrary.IsValid` _output_get_2)
      (if (and (`/Game/BubblePop_Template/Blueprints/BP_Bubble.Removed` _output_get_2) SkipRemoved)
        _
        (elif (or (not MatchType) (== (`/Game/BubblePop_Template/Blueprints/BP_Bubble.Type` (`local.CurrentTile`)) (`/Game/BubblePop_Template/Blueprints/BP_Bubble.Type` (`local.TargetTile`))))
          ;[1 1 1] Get Neighbors and add them to be processed
          (`KismetArrayLibrary.Array_Add` (`local.FoundCluster`) _currenttile)
          (bind _output_get_3 (set `local.Neighbors` (`self.GetNeighbors` _currenttile))) ; Find any neighbor bubble
          (for _array_element_2 _output_get_3
            (`/Engine/EditorBlueprintResources/StandardMacros.IsValid` _array_element_2
              (:`Is Valid`
                (if (not (`/Game/BubblePop_Template/Blueprints/BP_Bubble.Processed` _array_element_2))
                  (`KismetArrayLibrary.Array_Add` (`local.ToProcess`) _array_element_2)
                  (set `/Game/BubblePop_Template/Blueprints/BP_Bubble.Processed` true _array_element_2)))))))))
  (return (`local.FoundCluster`)))

(fn `FindFloatingCluster`
  (returns (Clusters :type "Array of /Game/BubblePop_Template/Blueprints/BP_Bubble Object Reference"))
  (locals (FoundCluster :type "Array of /Game/BubblePop_Template/Blueprints/BP_Bubble Object Reference") (FoundClusters :type "Array of /Game/BubblePop_Template/Blueprints/BP_Bubble Object Reference") (Tile :type "/Game/BubblePop_Template/Blueprints/BP_Bubble Object Reference") (Floating :type Boolean))
  ;[1 1 1] Search tiles to process
  (`self.ResetProcessed`) ; ResettingAnyProcessedBubble
  (for _index (range (+ (`/Game/BubblePop_Template/Blueprints/BP_Bubbles_Level.Columns` (`self.Level_Ref`)) 1))
    (for _index_2 (range (+ (`/Game/BubblePop_Template/Blueprints/BP_Bubbles_Level.Rows` (`self.Level_Ref`)) 1))
      (bind _returnvalue (`KismetMathLibrary.Conv_IntToDouble` _index))
      (bind _returnvalue_2 (`KismetMathLibrary.Conv_IntToDouble` _index_2))
      (bind _output_get (set `local.Tile` (`BlueprintMapLibrary.Map_Find` (`/Game/BubblePop_Template/Blueprints/BP_Bubbles_Level.Tile` (`self.Level_Ref`)) (`KismetMathLibrary.MakeVector2D` _returnvalue _returnvalue_2))))
      (`/Engine/EditorBlueprintResources/StandardMacros.IsValid` _output_get
        (:`Is Valid`
          (if (not (`/Game/BubblePop_Template/Blueprints/BP_Bubble.Processed` _output_get))
            ;[1 1 1] Add Any Floating Bubble
            (bind _output_get_2 (set `local.FoundCluster` (`self.FindCluster` _returnvalue _returnvalue_2 false false true))) ; Any neighbor found
            (if (not (<= (`KismetArrayLibrary.Array_Length` _output_get_2) 0))
              (set `local.Floating` true) ; Every one is meant to be floating
              (for _array_element (`local.FoundCluster`)
                (bind _gridposition_x (`KismetMathLibrary.BreakVector2D` (`/Game/BubblePop_Template/Blueprints/BP_Bubble.GridPosition` _array_element)))
                (if (== _gridposition_x (`KismetMathLibrary.Conv_IntToDouble` (`/Game/BubblePop_Template/Blueprints/BP_Bubbles_Level.Columns` (`self.Level_Ref`))))
                  (set `local.Floating` false)
                  (break)))
              (if (`local.Floating`)
                (`KismetArrayLibrary.Array_Append` (`local.FoundClusters`) (`local.FoundCluster`)))))))))
  (return (`local.FoundClusters`)) ; Returns any floating bubble found
)

(fn `GetNeighbors`
  (params (Bubble :type "/Game/BubblePop_Template/Blueprints/BP_Bubble Object Reference"))
  (returns (Neighbor :type "Array of /Game/BubblePop_Template/Blueprints/BP_Bubble Object Reference"))
  (locals (TileRow :type "Float (double-precision)") (N :type "Array of Vector2D Structure") (nX :type "Float (double-precision)") (nY :type "Float (double-precision)") (Neighbors :type "Array of /Game/BubblePop_Template/Blueprints/BP_Bubble Object Reference"))
  (bind (_gridposition_x _gridposition_y) (`KismetMathLibrary.BreakVector2D` (`/Game/BubblePop_Template/Blueprints/BP_Bubble.GridPosition` Bubble)))
  (bind (_gridposition_x_2 _gridposition_y_2) (`KismetMathLibrary.BreakVector2D` (`/Game/BubblePop_Template/Blueprints/BP_Bubble.GridPosition` Bubble)))
  (bind _nx (`local.nX`))
  (bind _level_ref (`self.Level_Ref`))
  (bind _ny (`local.nY`))
  (set `local.TileRow` (mod (+ _gridposition_y_2 (`KismetMathLibrary.Conv_IntToDouble` (`/Game/BubblePop_Template/Blueprints/BP_Bubbles_Level.RowOffset` (`self.Level_Ref`)))) 2.0)) ; Search if the tile is even or odd
  (if (== (`local.TileRow`) 0.0)
    (set `local.N` (`self.NeighborOffset_Odd`))
    (else
      (set `local.N` (`self.NeighborOffset_Even`))))
  (for _array_element (`local.N`)
    (bind (_x _y) (`KismetMathLibrary.BreakVector2D` _array_element))
    (set `local.nX` (+ _gridposition_x _x)) ; Neighbor X
    (set `local.nY` (+ _gridposition_y _y)) ; Neighbor Y
    (if (and (>= _nx 0.0) (<= _nx (`KismetMathLibrary.Conv_IntToDouble` (`/Game/BubblePop_Template/Blueprints/BP_Bubbles_Level.Columns` _level_ref))) (>= _ny 0.0) (<= _ny (`KismetMathLibrary.Conv_IntToDouble` (`/Game/BubblePop_Template/Blueprints/BP_Bubbles_Level.Rows` _level_ref))))
      (`KismetArrayLibrary.Array_Add` (`local.Neighbors`) (`BlueprintMapLibrary.Map_Find` (`/Game/BubblePop_Template/Blueprints/BP_Bubbles_Level.Tile` (`self.Level_Ref`)) (`KismetMathLibrary.MakeVector2D` (`local.nX`) (`local.nY`)))) ; Add the neighbor found to the array
    ))
  (return (`local.Neighbors`)))

(fn `UserConstructionScript`)