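; BP_Bubble is the bubble projectile for the BubblePop template, travelling at a set angle and speed once fired.
; Tick moves it, flips the angle to bounce off the Y bounds, and calls the level reference's SnapBubble upon reaching LevelX.
; FindCollisions scans every occupied grid tile with a manual circle-distance test instead of engine overlaps, stopping and snapping the bubble on the first hit.
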(event `self.ReceiveTick`
  (params (DeltaSeconds :type "Float (single-precision)"))
  (bind (_returnvalue_x _returnvalue_y _returnvalue_z) (`KismetMathLibrary.BreakVector` (`self.K2_GetActorLocation`)))
  (bind (_returnvalue_x_2 _returnvalue_y_2) (`KismetMathLibrary.BreakVector` (`self.K2_GetActorLocation`)))
  (bind (_returnvalue_x_3 _returnvalue_y_3 _returnvalue_z_2) (`KismetMathLibrary.BreakVector` (`self.K2_GetActorLocation`)))
  (bind _speed (`self.Speed`))
  (bind _level_ref (`self.Level_Ref`))
  (if (`self.bFired`)
    (`self.K2_AddActorLocalOffset` (`KismetMathLibrary.MakeVector` (* DeltaSeconds _speed (`KismetMathLibrary.Cos` (`KismetMathLibrary.DegreesToRadians` (`self.Angle`)))) (* DeltaSeconds _speed (`KismetMathLibrary.Sin` (`KismetMathLibrary.DegreesToRadians` (`self.Angle`))) -1.0)))
    (`self.Find Collisions`)
    (if (<= _returnvalue_y_2 0.0)
      (set `self.Angle` (* (`self.Angle`) -1.0))
      (`self.K2_SetActorLocation` (`KismetMathLibrary.MakeVector` _returnvalue_x_3 0.0 _returnvalue_z_2))
      (elif (>= _returnvalue_y_2 (`/Game/BubblePop_Template/Blueprints/BP_Bubbles_Level.LevelY` _level_ref))
        (set `self.Angle` (* (`self.Angle`) -1.0))
        (`self.K2_SetActorLocation` (`KismetMathLibrary.MakeVector` _returnvalue_x (`/Game/BubblePop_Template/Blueprints/BP_Bubbles_Level.LevelY` (`self.Level_Ref`)) _returnvalue_z))))
    (if (<= (`/Game/BubblePop_Template/Blueprints/BP_Bubbles_Level.LevelX` _level_ref) _returnvalue_x_2)
      (set `self.bFired` false)
      (`/Game/BubblePop_Template/Blueprints/BP_Bubbles_Level.SnapBubble` (`self.Level_Ref`) self))))

(fn `Circle Intersections`
  (params (x1 :type "Float (double-precision)") (y1 :type "Float (double-precision)") (r1 :type "Float (double-precision)") (x2 :type "Float (double-precision)") (y2 :type "Float (double-precision)") (r2 :type "Float (double-precision)"))
  (returns (Return :type Boolean))
  (locals (dx :type "Float (double-precision)") (dy :type "Float (double-precision)") (len :type "Float (double-precision)"))
  (set `local.dx` (- x1 x2))
  (set `local.dy` (- y1 y2))
  (bind _output_get (set `local.len` (`KismetMathLibrary.Sqrt` (+ (* (`local.dx`) (`local.dx`)) (* (`local.dy`) (`local.dy`))))))
  (return (< _output_get (+ r1 r2))))

(fn `Find Collisions`
  (locals (Local_Tile :type "Map of Vector2D Structure to /Game/BubblePop_Template/Blueprints/BP_Bubble Object Reference") (Local_Coor :type "Vector2D Structure"))
  (bind (_returnvalue_x _returnvalue_y) (`KismetMathLibrary.BreakVector` (`self.K2_GetActorLocation`)))
  (bind (_local_coor_x _local_coor_y) (`KismetMathLibrary.BreakVector2D` (`local.Local_Coor`)))
  (bind _level_ref (`self.Level_Ref`))
  (bind _radius (`/Game/BubblePop_Template/Blueprints/BP_Bubbles_Level.Radius` _level_ref))
  (bind _returnvalue (`KismetMathLibrary.Conv_IntToDouble` (/ (`/Game/BubblePop_Template/Blueprints/BP_Bubbles_Level.TileWidth` _level_ref) 2)))
  (bind _returnvalue_2 (`KismetMathLibrary.Conv_IntToDouble` (/ (`/Game/BubblePop_Template/Blueprints/BP_Bubbles_Level.RowHeight` _level_ref) 2)))
  (for _index (range (+ (`/Game/BubblePop_Template/Blueprints/BP_Bubbles_Level.Rows` (`self.Level_Ref`)) 1))
    (for _index_2 (range (+ (`/Game/BubblePop_Template/Blueprints/BP_Bubbles_Level.Columns` (`self.Level_Ref`)) 1))
      (if (`KismetSystemLibrary.IsValid` (`BlueprintMapLibrary.Map_Find` (`/Game/BubblePop_Template/Blueprints/BP_Bubbles_Level.Tile` (`self.Level_Ref`)) (`KismetMathLibrary.MakeVector2D` (`KismetMathLibrary.Conv_IntToDouble` _index_2) (`KismetMathLibrary.Conv_IntToDouble` _index))))
        (bind (_tile_x _tile_y) (`/Game/BubblePop_Template/Blueprints/BP_Bubbles_Level.GetTileCoordinate` (`self.Level_Ref`) _index_2 _index))
        (set `local.Local_Coor` (`KismetMathLibrary.MakeVector2D` (`KismetMathLibrary.Conv_IntToDouble` _tile_x) (`KismetMathLibrary.Conv_IntToDouble` _tile_y)))
        (if (`self.Circle Intersections` (+ _returnvalue_x _returnvalue_2) (+ _returnvalue_y _returnvalue) _radius (+ _local_coor_x _returnvalue) (+ _local_coor_y _returnvalue_2) _radius)
          (set `self.bFired` false)
          (`/Game/BubblePop_Template/Blueprints/BP_Bubbles_Level.SnapBubble` (`self.Level_Ref`) self)
          (return))))))

(fn `UserConstructionScript`)