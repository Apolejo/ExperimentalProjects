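; Controller actor for a bubble-pop game that builds the level and links it to the player on BeginPlay.
; It spawns a BP_Bubbles_Level grid, then cross-references it with the BP_PlayerWeapon pawn and sets the pawn's Y to half the level's LevelY.
; Both grid and weapon receive the same random color limit.
; GameOver and GameWon are placeholder events that both print "GameOver".
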(event `self.ReceiveBeginPlay`
  (bind _returnvalue (`|SpawnActorFromClass` "/Game/BubblePop_Template/Blueprints/BP_Bubbles_Level.BP_Bubbles_Level_C" (`KismetMathLibrary.MakeTransform` (0.0 0.0 0.0)) "Undefined" "OverrideRootScale" null 100 100 0 10 15 5 3 (`self.CustomTile`) false (`self.BubbleRandomColors`) null))
  (bind _output_get (set `self.TileGrid` _returnvalue))
  (bind _asbp_player_weapon (cast `/Game/BubblePop_Template/Blueprints/BP_PlayerWeapon` (`GameplayStatics.GetPlayerPawn` 0)))
  (set `/Game/BubblePop_Template/Blueprints/BP_PlayerWeapon.Level_Ref` _output_get _asbp_player_weapon)
  (set `/Game/BubblePop_Template/Blueprints/BP_Bubbles_Level.PlayerActor` _asbp_player_weapon _output_get)
  (`self.K2_SetActorLocation` _asbp_player_weapon (`KismetMathLibrary.MakeVector` 0.0 (/ (`/Game/BubblePop_Template/Blueprints/BP_Bubbles_Level.LevelY` (`self.TileGrid`)) 2.0)) false false)
  (set `/Game/BubblePop_Template/Blueprints/BP_PlayerWeapon.PlayerMaxColorSpawn` (`self.BubbleRandomColors`) _asbp_player_weapon))

(event `GameOver`
  (`KismetSystemLibrary.PrintString` "GameOver" true true (struct :`R` 1.0 :`B` 0.321772 :`A` 1.0) 10.0))

(event `GameWon`
  (`KismetSystemLibrary.PrintString` "GameOver" true true (struct :`R` 1.0 :`B` 0.321772 :`A` 1.0) 10.0))

(fn `UserConstructionScript`)